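; BP_HealStone is an interactable heal stone that shows an interaction prompt when Kratos comes near; no healing logic is in this Blueprint.
; Its SphereComp overlap events cast the other actor to BP_Kratos, reach its WBP_MainUI, and show PressEButton on entering and hide it on leaving.
; The other event stubs and the construction script are empty.
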(event `self.SphereComp.OnComponentBeginOverlap`
  (params (OverlappedComponent :type "PrimitiveComponent Object Reference") (OtherActor :type "Actor Object Reference") (OtherComp :type "PrimitiveComponent Object Reference") (OtherBodyIndex :type Integer) (bFromSweep :type Boolean) (SweepResult :type "HitResult Structure (by ref)"))
  (bind _asbp_kratos (cast `/Game/AHS/Blueprints/BP_Kratos` OtherActor))
  (bind _aswbp_main_ui (cast `/Game/AHS/UI/WBP_MainUI` (`KratosCharacter.MainUI` _asbp_kratos)))
  (`Widget.SetVisibility` (`/Game/AHS/UI/WBP_MainUI.PressEButton` _aswbp_main_ui) "Visible"))

(event `self.SphereComp.OnComponentEndOverlap`
  (params (OverlappedComponent :type "PrimitiveComponent Object Reference") (OtherActor :type "Actor Object Reference") (OtherComp :type "PrimitiveComponent Object Reference") (OtherBodyIndex :type Integer))
  (bind _asbp_kratos (cast `/Game/AHS/Blueprints/BP_Kratos` OtherActor))
  (bind _aswbp_main_ui (cast `/Game/AHS/UI/WBP_MainUI` (`KratosCharacter.MainUI` _asbp_kratos)))
  (`Widget.SetVisibility` (`/Game/AHS/UI/WBP_MainUI.PressEButton` _aswbp_main_ui) "Hidden"))

(fn `UserConstructionScript`)
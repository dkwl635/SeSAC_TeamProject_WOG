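; Game mode Blueprint that handles level audio, input setup and an on-screen Thor text.
; BeginPlay spawns and stores background music and thunder sounds, then switches to game-only input with the cursor hidden.
; BGM_Off stops both sounds and destroys every BP_MapLighjting actor.
; SetThorText lazily creates a WBP_EndText widget, adds it to the viewport and updates its text.
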(event `self.ReceiveBeginPlay`
  (bind _returnvalue (`GameplayStatics.GetPlayerController` 0))
  (bind _returnvalue_2 (`GameplayStatics.SpawnSoundAtLocation` "/Game/KJW/SC_BGM.SC_BGM" (0.0 0.0 0.0) (struct) 1.0 1.0 0.0 null null))
  (set `self.BGM` _returnvalue_2)
  (bind _returnvalue_3 (`GameplayStatics.SpawnSoundAtLocation` "/Game/KJW/SC_Thunder_Sounds.SC_Thunder_Sounds" (0.0 0.0 0.0) (struct) 1.0 1.0 0.0 null null))
  (set `self.BGM_Effect` _returnvalue_3)
  (`WidgetBlueprintLibrary.SetInputMode_GameOnly` _returnvalue)
  (set `PlayerController.bShowMouseCursor` false _returnvalue))

(event `BGM_Off`
  (`KismetSystemLibrary.PrintString` "Hello")
  (`AudioComponent.Stop` (`self.BGM`))
  (`AudioComponent.Stop` (`self.BGM_Effect`))
  (bind _outactors (`GameplayStatics.GetAllActorsOfClass` "/Game/KJW/Blueprint/BP_MapLighjting.BP_MapLighjting_C"))
  (for _array_element _outactors
    (`self.K2_DestroyActor` _array_element)))

(event `SetThorText`
  (params (TextValue :type Text))
  (bind _thortextwbp (`self.ThorTextWBP`)
    (:`then`
      _)
    (:`else`
      (bind _returnvalue (`|CreateWidget` "/Game/KJW/WBP_EndText.WBP_EndText_C"))
      (bind _output_get (set `self.ThorTextWBP` _returnvalue))
      (`UserWidget.AddToViewport` _output_get 0)))
  (`/Game/KJW/WBP_EndText.SetText` _thortextwbp TextValue))

(fn `UserConstructionScript`)
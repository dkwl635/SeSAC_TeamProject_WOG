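; Anim notify state that forwards animation timing windows to the Thor character for its attack or behavior patterns.
; On begin it casts the mesh owner to Thor, caches it, and calls NotifyBeginPattern with its EventIndex and total duration.
; Tick and end calls relay the same EventIndex, plus frame delta on tick, to the cached Thor's matching pattern handlers.
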(fn `Received_NotifyBegin`
  (params (MeshComp :type "SkeletalMeshComponent Object Reference") (Animation :type "AnimSequenceBase Object Reference") (TotalDuration :type "Float (single-precision)") (EventReference :type "AnimNotifyEventReference Structure (by ref)"))
  (returns (ReturnValue :type Boolean))
  (bind _returnvalue (`ActorComponent.GetOwner` MeshComp))
  (`/Engine/EditorBlueprintResources/StandardMacros.IsValid` _returnvalue
    (:`Is Valid`
      (bind _asthor (cast `Thor` _returnvalue)
        (:`then`
          (`self.SetThor` _asthor)
          (`Thor.NotifyBeginPattern` (`self.Thor`) (`self.EventIndex`) TotalDuration)
          (return true))
        (:`CastFailed`
          _)))
    (:`Is Not Valid`
      _))
  (return false))

(fn `Received_NotifyEnd`
  (params (MeshComp :type "SkeletalMeshComponent Object Reference") (Animation :type "AnimSequenceBase Object Reference") (EventReference :type "AnimNotifyEventReference Structure (by ref)"))
  (returns (ReturnValue :type Boolean))
  (bind _thor (`self.Thor`))
  (`/Engine/EditorBlueprintResources/StandardMacros.IsValid` _thor
    (:`Is Valid`
      (`Thor.NotifyEndPattrern` _thor (`self.EventIndex`))
      (return true))
    (:`Is Not Valid`
      (return false))))

(fn `Received_NotifyTick`
  (params (MeshComp :type "SkeletalMeshComponent Object Reference") (Animation :type "AnimSequenceBase Object Reference") (FrameDeltaTime :type "Float (single-precision)") (EventReference :type "AnimNotifyEventReference Structure (by ref)"))
  (returns (ReturnValue :type Boolean))
  (bind _thor (`self.Thor`))
  (`/Engine/EditorBlueprintResources/StandardMacros.IsValid` _thor
    (:`Is Valid`
      (`Thor.NotifyTickPattrern` _thor (`self.EventIndex`) FrameDeltaTime)
      (return true))
    (:`Is Not Valid`
      (return false))))
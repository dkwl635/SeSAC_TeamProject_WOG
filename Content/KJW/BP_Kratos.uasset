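; Player Kratos character Blueprint for a fight against Thor, who is found at BeginPlay and set as the lock-on target.
; Tick turns control rotation toward that target; Tab toggles lock-on and aiming suspends it.
; Attack input plays axe or punch combo montages, using notifies and input-refreshed counters to continue or stop them, while fist and axe overlaps feed OnHandOverlapBP.
; Events handle axe socketing and throw visibility, and debug keys force Thor's patterns.
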(event OnComponentBeginOverlap(Fist_L)
  (params (OverlappedComponent :type Primitive%20Component%20Object%20Reference) (OtherActor :type Actor%20Object%20Reference) (OtherComp :type Primitive%20Component%20Object%20Reference) (OtherBodyIndex :type Integer) (bFromSweep :type Boolean) (SweepResult :type Hit%20Result%20Structure%20%28by%20ref%29))
  ;[0.15 0.15 0.15 0.5] 주먹 충돌(Collision)
  (Class|KratosCharacter|OnHandOverlapBP OtherActor (.location SweepResult)))

(event OnComponentBeginOverlap(Fist_R)
  (params (OverlappedComponent :type Primitive%20Component%20Object%20Reference) (OtherActor :type Actor%20Object%20Reference) (OtherComp :type Primitive%20Component%20Object%20Reference) (OtherBodyIndex :type Integer) (bFromSweep :type Boolean) (SweepResult :type Hit%20Result%20Structure%20%28by%20ref%29))
  ;[0.15 0.15 0.15 0.5] 주먹 충돌(Collision)
  (Class|KratosCharacter|OnHandOverlapBP OtherActor (.location SweepResult)))

(event OnComponentBeginOverlap(AxeCollision)
  (params (OverlappedComponent :type Primitive%20Component%20Object%20Reference) (OtherActor :type Actor%20Object%20Reference) (OtherComp :type Primitive%20Component%20Object%20Reference) (OtherBodyIndex :type Integer) (bFromSweep :type Boolean) (SweepResult :type Hit%20Result%20Structure%20%28by%20ref%29))
  ;[0.15 0.15 0.15 0.5] 주먹 충돌(Collision)
  (Class|KratosCharacter|OnHandOverlapBP OtherActor (.location SweepResult)))

(event Custom|Hold%20Weapon%20in%20Hand
  ;[0.15 0.15 0.15 0.5] 무기 장착 및 도끼 던지기 애니메이션 실행
  (Transformation|AttachComponentToComponent (Variables|Default|GetAxeMesh) (Variables|Character|GetMesh) "Armmed" "KeepRelative" "KeepRelative" "KeepRelative" true))

(event Custom|UnHold%20Weapon%20in%20Hand
  ;[0.15 0.15 0.15 0.5] 무기 장착 및 도끼 던지기 애니메이션 실행
  (Transformation|AttachComponentToComponent (Variables|Default|GetAxeMesh) (Variables|Character|GetMesh) "Unarmmed" "KeepRelative" "KeepRelative" "KeepRelative" true))

(event Custom|Throw%20Weapon
  ;[0.15 0.15 0.15 0.5] 무기 장착 및 도끼 던지기 애니메이션 실행
  (Rendering|SetVisibility (Variables|Default|GetAxeMesh) false false))

(event Custom|GetBackWeapon
  ;[0.15 0.15 0.15 0.5] 무기 장착 및 도끼 던지기 애니메이션 실행
  (Rendering|SetVisibility (Variables|Default|GetAxeMesh) true false))

(event Input|EnhancedActionEvents|EnhancedInputActionIA_Aim
  (params (ActionValue :type Boolean) (ElapsedSeconds :type Float%20%28double-precision%29) (TriggeredSeconds :type Float%20%28double-precision%29) (InputAction :type Input%20Action%20Object%20Reference :default "/Game/AHS/Inputs/IA_Aim.IA_Aim"))
  (:Started
    (Variables|Default|SetTargetLock false)
    (Variables|Default|SetLockOnTarget 0))
  (:Completed
    (Variables|Default|SetTargetLock true)
    (Variables|Default|SetLockOnTarget (Variables|Default|GetTHOR))))

(event Input|EnhancedActionEvents|EnhancedInputActionIA_KratosAttack
  (params (ActionValue :type Boolean) (ElapsedSeconds :type Float%20%28double-precision%29) (TriggeredSeconds :type Float%20%28double-precision%29) (InputAction :type Input%20Action%20Object%20Reference :default "/Game/AHS/Inputs/IA_KratosAttack.IA_KratosAttack"))
  (:Started
    (if (Variables|Default|GetKratos_EquippedWeapon)
      ;[0.15 0.15 0.15 0.5] 도끼 콤보
      (if (not (Animation|Montage|MontageIsPlaying (Components|SkeletalMesh|GetAnimInstance (Variables|Character|GetMesh)) "/Game/AHS/Assets/Mixamo/Kratos_Animations/ComboAttack_AnimMontage.ComboAttack_AnimMontage"))
        (Animation|Montage|PlayMontage (Variables|Character|GetMesh) "/Game/AHS/Assets/Mixamo/Kratos_Animations/ComboAttack_AnimMontage.ComboAttack_AnimMontage"
          (:OnNotifyBegin
            (bind _result (Math|Integer|DecrementInt (Variables|Default|GetattackIndex))
              (:%20%20
                (if (< _result 0)
                  (Animation|Montage|MontageStop (Components|SkeletalMesh|GetAnimInstance (Variables|Character|GetMesh)) 0.75 "/Game/AHS/Assets/Mixamo/Kratos_Animations/ComboAttack_AnimMontage.ComboAttack_AnimMontage"))))))
        (else
          (Variables|Default|SetattackIndex 1)))
      (else
        ;[0.15 0.15 0.15 0.5] 도끼 콤보
        (if (not (Animation|Montage|MontageIsPlaying (Components|SkeletalMesh|GetAnimInstance (Variables|Character|GetMesh)) "/Game/AHS/Animations/AM_PunchCombo_Kratos.AM_PunchCombo_Kratos"))
          (Animation|Montage|PlayMontage (Variables|Character|GetMesh) "/Game/AHS/Animations/AM_PunchCombo_Kratos.AM_PunchCombo_Kratos"
            (:OnNotifyBegin
              (bind _result_2 (Math|Integer|DecrementInt (Variables|Default|GetattackIndex2))
                (:%20%20
                  (if (< _result_2 0)
                    (Animation|Montage|MontageStop (Components|SkeletalMesh|GetAnimInstance (Variables|Character|GetMesh)) 0.75 "/Game/AHS/Animations/AM_PunchCombo_Kratos.AM_PunchCombo_Kratos"))))))
          (else
            (Variables|Default|SetattackIndex2 1)))))))

(event EventBeginPlay
  ;[0.15 0.15 0.15 0.5] Basic
  (bind _returnvalue (Actor|GetActorOfClass "/Game/KJW/Blueprint/BP_Thor.BP_Thor_C"))
  (Variables|Default|SetTHOR _returnvalue)
  (Variables|Default|SetLockOnTarget (Variables|Default|GetTHOR)))

(event Collision|EventActorBeginOverlap
  (params (OtherActor :type Actor%20Object%20Reference))
  ;[0.15 0.15 0.15 0.5] Basic
)

(event EventTick
  (params (DeltaSeconds :type Float%20%28single-precision%29))
  ;[0.15 0.15 0.15 0.5] 카메라 록온을 위해 Tick에 구현
  (Variables|Default|GetLockOnTarget
    (:then
      (Pawn|SetControlRotation (Pawn|GetController) (Math|Rotator|FindLookatRotation (Transformation|GetActorLocation) (Transformation|GetActorLocation (Variables|Default|GetLockOnTarget)))))
    (:else)))

(event Input|KeyboardEvents|DebugKeyM
  (params (Key :type Key%20Structure) (ActionValue :type Input%20Action%20Value%20Structure))
  (bind _thor (Variables|Default|GetTHOR))
  ;[0.15 0.15 0.15 0.5] 임시 토르 조정
  (:Pressed
    (Utilities|IsValid _thor
      (:Is%20Valid
        (Class|Thor|ChangePattarn _thor "ATTACK_THUNDER_CLAP")))))

(event Input|KeyboardEvents|DebugKeyX
  (params (Key :type Key%20Structure) (ActionValue :type Input%20Action%20Value%20Structure))
  (bind _thor (Variables|Default|GetTHOR))
  ;[0.15 0.15 0.15 0.5] 임시 토르 조정
  (:Pressed
    (Utilities|IsValid _thor
      (:Is%20Valid
        (Class|Thor|ChangePattarn _thor "ATTACK_TRIPLE_LIGHTING_STRIKES")))))

(event Input|KeyboardEvents|DebugKeyN
  (params (Key :type Key%20Structure) (ActionValue :type Input%20Action%20Value%20Structure))
  (bind _thor (Variables|Default|GetTHOR))
  ;[0.15 0.15 0.15 0.5] 임시 토르 조정
  (:Pressed
    (Utilities|IsValid _thor
      (:Is%20Valid
        (Class|Thor|ChangePattarn _thor "ATTACK_TRIPLE_STRIKE_COMBO")))))

(event Input|KeyboardEvents|DebugKeyB
  (params (Key :type Key%20Structure) (ActionValue :type Input%20Action%20Value%20Structure))
  (bind _thor (Variables|Default|GetTHOR))
  ;[0.15 0.15 0.15 0.5] 임시 토르 조정
  (:Pressed
    (Utilities|IsValid _thor
      (:Is%20Valid
        (Class|Thor|ChangePattarn _thor "ATTACK_HAMMER_THROW_START")))))

(event Input|KeyboardEvents|DebugKeyV
  (params (Key :type Key%20Structure) (ActionValue :type Input%20Action%20Value%20Structure))
  (bind _thor (Variables|Default|GetTHOR))
  ;[0.15 0.15 0.15 0.5] 임시 토르 조정
  (:Pressed
    (Utilities|IsValid _thor
      (:Is%20Valid
        (Class|Thor|ChangePattarn _thor "ATTACK_HAMMER_THROW_END")))))

(event Input|KeyboardEvents|DebugKeyC
  (params (Key :type Key%20Structure) (ActionValue :type Input%20Action%20Value%20Structure))
  (bind _thor (Variables|Default|GetTHOR))
  ;[0.15 0.15 0.15 0.5] 임시 토르 조정
  (:Pressed
    (Utilities|IsValid _thor
      (:Is%20Valid
        (Class|Thor|ChangePattarn _thor "ATTACK_TRIPLE_HAMMER_STRIKES")))))

(event Input|KeyboardEvents|DebugKeyL
  (params (Key :type Key%20Structure) (ActionValue :type Input%20Action%20Value%20Structure))
  (bind _thor (Variables|Default|GetTHOR))
  ;[0.15 0.15 0.15 0.5] 임시 토르 조정
  (:Pressed
    (Utilities|IsValid _thor
      (:Is%20Valid
        (Class|Thor|ChangePattarn _thor "HIT")))))

(event Input|KeyboardEvents|Tab
  (params (Key :type Key%20Structure))
  ;[0.15 0.15 0.15 0.5] 카메라 록온
  (:Pressed
    (Utilities|FlowControl|FlipFlop
      (:A
        (Variables|Default|SetLockOnTarget (Variables|Default|GetTHOR)))
      (:B
        (Variables|Default|SetLockOnTarget 0)))))

(event Input|KeyboardEvents|SpaceBar
  (params (Key :type Key%20Structure))
  (:Pressed
    (if (Variables|Default|GetKratos_EquippedWeapon)
      ;[0.15 0.15 0.15 0.5] 도끼 콤보
      (if (not (Animation|Montage|MontageIsPlaying (Components|SkeletalMesh|GetAnimInstance (Variables|Character|GetMesh)) "/Game/AHS/Assets/Mixamo/Kratos_Animations/ComboAttack_AnimMontage.ComboAttack_AnimMontage"))
        (Animation|Montage|PlayMontage (Variables|Character|GetMesh) "/Game/AHS/Assets/Mixamo/Kratos_Animations/ComboAttack_AnimMontage.ComboAttack_AnimMontage"
          (:OnNotifyBegin
            (bind _result (Math|Integer|DecrementInt (Variables|Default|GetattackIndex))
              (:%20%20
                (if (< _result 0)
                  (Animation|Montage|MontageStop (Components|SkeletalMesh|GetAnimInstance (Variables|Character|GetMesh)) 0.75 "/Game/AHS/Assets/Mixamo/Kratos_Animations/ComboAttack_AnimMontage.ComboAttack_AnimMontage"))))))
        (else
          (Variables|Default|SetattackIndex 1)))
      (else
        ;[0.15 0.15 0.15 0.5] 도끼 콤보
        (if (not (Animation|Montage|MontageIsPlaying (Components|SkeletalMesh|GetAnimInstance (Variables|Character|GetMesh)) "/Game/AHS/Animations/AM_PunchCombo_Kratos.AM_PunchCombo_Kratos"))
          (Animation|Montage|PlayMontage (Variables|Character|GetMesh) "/Game/AHS/Animations/AM_PunchCombo_Kratos.AM_PunchCombo_Kratos"
            (:OnNotifyBegin
              (bind _result_2 (Math|Integer|DecrementInt (Variables|Default|GetattackIndex2))
                (:%20%20
                  (if (< _result_2 0)
                    (Animation|Montage|MontageStop (Components|SkeletalMesh|GetAnimInstance (Variables|Character|GetMesh)) 0.75 "/Game/AHS/Animations/AM_PunchCombo_Kratos.AM_PunchCombo_Kratos"))))))
          (else
            (Variables|Default|SetattackIndex2 1)))))))

(fn ConstructionScript)
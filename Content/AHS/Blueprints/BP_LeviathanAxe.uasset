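; BP_LeviathanAxe is the Leviathan Axe actor for Kratos, handling attack overlaps and thrown movement.
; AxeAttack overlaps pass the other actor and impact point to OnAxeOverlapBP, which is defined outside these graphs.
; ThrowAxe moves the axe without sweep by Speed and DeltaTime along the player BP_Kratos camera's current forward vector, so each call follows where the camera points.
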(event `self.ReceiveTick`
  (params (DeltaSeconds :type "Float (single-precision)")))

(event `self.Axe Attack.OnComponentBeginOverlap`
  (params (OverlappedComponent :type "PrimitiveComponent Object Reference") (OtherActor :type "Actor Object Reference") (OtherComp :type "PrimitiveComponent Object Reference") (OtherBodyIndex :type Integer) (bFromSweep :type Boolean) (SweepResult :type "HitResult Structure (by ref)"))
  (`self.OnAxeOverlapBP` OtherActor SweepResult_ImpactPoint))

(fn `ThrowAxe`
  (params (DeltaTime :type "Float (double-precision)"))
  ; 방향
  (bind _asbp_kratos (cast `/Game/AHS/Blueprints/BP_Kratos` (`GameplayStatics.GetPlayerCharacter` 0)))
  (`self.K2_SetActorLocation` (+ (`self.K2_GetActorLocation`) (* (`SceneComponent.GetForwardVector` (`KratosCharacter.KratosCamComp` _asbp_kratos)) (`self.Speed`) DeltaTime))))

(fn `UserConstructionScript`)
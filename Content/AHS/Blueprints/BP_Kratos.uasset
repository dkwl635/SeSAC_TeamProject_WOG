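; Kratos player character Blueprint handling camera lock-on, Leviathan Axe visuals and fist hit detection.
; Tab sphere-traces along the camera direction for a pawn that Tick keeps the controller facing, until Tab or aiming clears it.
; Events swap the axe between sockets or toggle its visibility for throws, while fist overlaps call OnHandOverlapBP.
; Debug keys force BP_Thor attack patterns; the axe and punch combo montage logic is disconnected.
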(event OnComponentBeginOverlap(Fist_L)
  (params (OverlappedComponent :type Primitive%20Component%20Object%20Reference) (OtherActor :type Actor%20Object%20Reference) (OtherComp :type Primitive%20Component%20Object%20Reference) (OtherBodyIndex :type Integer) (bFromSweep :type Boolean) (SweepResult :type Hit%20Result%20Structure%20%28by%20ref%29))
  ;[0.15 0.15 0.15 0.5] 주먹 충돌(Collision)
  (Class|KratosCharacter|OnHandOverlapBP OtherActor (.location SweepResult)))

(event OnComponentBeginOverlap(Fist_R)
  (params (OverlappedComponent :type Primitive%20Component%20Object%20Reference) (OtherActor :type Actor%20Object%20Reference) (OtherComp :type Primitive%20Component%20Object%20Reference) (OtherBodyIndex :type Integer) (bFromSweep :type Boolean) (SweepResult :type Hit%20Result%20Structure%20%28by%20ref%29))
  ;[0.15 0.15 0.15 0.5] 주먹 충돌(Collision)
  (Class|KratosCharacter|OnHandOverlapBP OtherActor (.location SweepResult)))

(event Custom|Hold%20Weapon%20in%20Hand
  ;[0.15 0.15 0.15 0.5] 무기 장착 및 도끼 던지기 애니메이션 실행
  (Transformation|AttachComponentToComponent (Variables|Default|GetBP_LeviathanAxe) (Variables|Character|GetMesh) "Armmed" "KeepRelative" "KeepRelative" "KeepRelative" true))

(event Custom|UnHold%20Weapon%20in%20Hand
  ;[0.15 0.15 0.15 0.5] 무기 장착 및 도끼 던지기 애니메이션 실행
  (Transformation|AttachComponentToComponent (Variables|Default|GetBP_LeviathanAxe) (Variables|Character|GetMesh) "Unarmmed" "KeepRelative" "KeepRelative" "KeepRelative" true))

(event Custom|Throw%20Weapon
  ;[0.15 0.15 0.15 0.5] 무기 장착 및 도끼 던지기 애니메이션 실행
  (Rendering|SetVisibility (Variables|Default|GetBP_LeviathanAxe) false false))

(event Custom|GetBackWeapon
  ;[0.15 0.15 0.15 0.5] 무기 장착 및 도끼 던지기 애니메이션 실행
  (Rendering|SetVisibility (Variables|Default|GetBP_LeviathanAxe) true false))

(event Input|EnhancedActionEvents|EnhancedInputActionIA_Aim
  (params (ActionValue :type Boolean) (ElapsedSeconds :type Float%20%28double-precision%29) (TriggeredSeconds :type Float%20%28double-precision%29) (InputAction :type Input%20Action%20Object%20Reference :default "/Game/AHS/Inputs/IA_Aim.IA_Aim"))
  (:Started
    (Variables|Default|SetTargetLock false)
    (Variables|Default|SetHit%20Target 0)))

(event Input|EnhancedActionEvents|EnhancedInputActionIA_KratosAttack
  (params (ActionValue :type Boolean) (ElapsedSeconds :type Float%20%28double-precision%29) (TriggeredSeconds :type Float%20%28double-precision%29) (InputAction :type Input%20Action%20Object%20Reference :default "/Game/AHS/Inputs/IA_KratosAttack.IA_KratosAttack")))

(event EventBeginPlay
  ;[0.15 0.15 0.15 0.5] Basic
  (bind _returnvalue (Actor|GetActorOfClass "/Game/KJW/Blueprint/BP_Thor.BP_Thor_C"))
  (Variables|Default|SetNewVar _returnvalue))

(event Collision|EventActorBeginOverlap
  (params (OtherActor :type Actor%20Object%20Reference))
  ;[0.15 0.15 0.15 0.5] Basic
)

(event EventTick
  (params (DeltaSeconds :type Float%20%28single-precision%29))
  ;[0.15 0.15 0.15 0.5] 카메라 록온을 위해 Tick에 구현
  (Variables|Default|GetHit%20Target
    (:then
      (Pawn|SetControlRotation (Pawn|GetController) (Math|Rotator|FindLookatRotation (Transformation|GetActorLocation) (Transformation|GetActorLocation (Variables|Default|GetHit%20Target)))))
    (:else)))

(event Input|KeyboardEvents|DebugKeyM
  (params (Key :type Key%20Structure :default "None") (ActionValue :type Input%20Action%20Value%20Structure))
  (bind _newvar (Variables|Default|GetNewVar))
  ;[0.15 0.15 0.15 0.5] 임시 토르 조정
  (:Pressed
    (Utilities|IsValid _newvar
      (:Is%20Valid
        (Class|Thor|ChangePattarn _newvar "ATTACK_THUNDER_CLAP")))))

(event Input|KeyboardEvents|DebugKeyX
  (params (Key :type Key%20Structure :default "None") (ActionValue :type Input%20Action%20Value%20Structure))
  (bind _newvar (Variables|Default|GetNewVar))
  ;[0.15 0.15 0.15 0.5] 임시 토르 조정
  (:Pressed
    (Utilities|IsValid _newvar
      (:Is%20Valid
        (Class|Thor|ChangePattarn _newvar "ATTACK_TRIPLE_LIGHTING_STRIKES")))))

(event Input|KeyboardEvents|DebugKeyN
  (params (Key :type Key%20Structure :default "None") (ActionValue :type Input%20Action%20Value%20Structure))
  (bind _newvar (Variables|Default|GetNewVar))
  ;[0.15 0.15 0.15 0.5] 임시 토르 조정
  (:Pressed
    (Utilities|IsValid _newvar
      (:Is%20Valid
        (Class|Thor|ChangePattarn _newvar "ATTACK_TRIPLE_STRIKE_COMBO")))))

(event Input|KeyboardEvents|DebugKeyB
  (params (Key :type Key%20Structure :default "None") (ActionValue :type Input%20Action%20Value%20Structure))
  (bind _newvar (Variables|Default|GetNewVar))
  ;[0.15 0.15 0.15 0.5] 임시 토르 조정
  (:Pressed
    (Utilities|IsValid _newvar
      (:Is%20Valid
        (Class|Thor|ChangePattarn _newvar "ATTACK_HAMMER_THROW_START")))))

(event Input|KeyboardEvents|DebugKeyV
  (params (Key :type Key%20Structure :default "None") (ActionValue :type Input%20Action%20Value%20Structure))
  (bind _newvar (Variables|Default|GetNewVar))
  ;[0.15 0.15 0.15 0.5] 임시 토르 조정
  (:Pressed
    (Utilities|IsValid _newvar
      (:Is%20Valid
        (Class|Thor|ChangePattarn _newvar "ATTACK_HAMMER_THROW_END")))))

(event Input|KeyboardEvents|DebugKeyC
  (params (Key :type Key%20Structure :default "None") (ActionValue :type Input%20Action%20Value%20Structure))
  (bind _newvar (Variables|Default|GetNewVar))
  ;[0.15 0.15 0.15 0.5] 임시 토르 조정
  (:Pressed
    (Utilities|IsValid _newvar
      (:Is%20Valid
        (Class|Thor|ChangePattarn _newvar "ATTACK_TRIPLE_HAMMER_STRIKES")))))

(event Input|KeyboardEvents|DebugKeyL
  (params (Key :type Key%20Structure :default "None") (ActionValue :type Input%20Action%20Value%20Structure))
  (bind _newvar (Variables|Default|GetNewVar))
  ;[0.15 0.15 0.15 0.5] 임시 토르 조정
  (:Pressed
    (Utilities|IsValid _newvar
      (:Is%20Valid
        (Class|Thor|ChangePattarn _newvar "HIT")))))

(event Input|KeyboardEvents|Tab
  (params (Key :type Key%20Structure :default "None"))
  (bind _returnvalue (Transformation|GetActorLocation))
  ;[0.15 0.15 0.15 0.5] 카메라 록온
  (:Pressed
    (Utilities|FlowControl|FlipFlop
      (:A
        (Variables|Default|SetTargetLock true)
        (bind (_outhit _returnvalue_2) (Collision|SphereTraceForObjects _returnvalue (+ _returnvalue (* (Math|Vector|GetForwardVector (Transformation|GetWorldRotation (Variables|Default|GetKratosCamComp))) 5e+02)) 125.0 (Utilities|Array|MakeArray "ObjectTypeQuery3") false 0 "ForDuration"))
        (if _returnvalue_2
          (Variables|Default|SetHit%20Target (.HitActor (Collision|BreakHitResult _outhit)))))
      (:B
        (Variables|Default|SetTargetLock false)
        (Variables|Default|SetHit%20Target 0)))))

(fn ConstructionScript)
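; BP_MapLighjting is an actor that produces recurring lightning strikes at random spots around the map.
; Tick accumulates a delay timer and, past its threshold, resets it to a random offset so strikes come every two to three seconds.
; Each strike moves the actor to random X/Y coordinates around the world origin, then calls Spawn.
; Spawn re-uses the actor's own components, activating the blue zap effect and playing the thunder sound.
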(event `self.ReceiveTick`
  (params (DeltaSeconds :type "Float (single-precision)"))
  (bind _output_get (set `self.MoveDelay` (+ DeltaSeconds (`self.MoveDelay`))))
  (if (>= _output_get 3.0)
    (set `self.MoveDelay` (`KismetMathLibrary.RandomFloatInRange` 0.0 1.0))
    (`self.K2_SetActorLocation` (`KismetMathLibrary.MakeVector` (`KismetMathLibrary.RandomFloatInRange` -1500.0 1500.0) (`KismetMathLibrary.RandomFloatInRange` -1500.0 1500.0)))
    (`self.Spawn`)))

(event `Spawn`
  (`ActorComponent.Activate` (`self.NS_Zap_02_Blue`) false)
  (`AudioComponent.Play` (`self.thunder`) 0.0))

(fn `UserConstructionScript`)